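; Game mode Blueprint (GM) that handles single-slot save and load of the player's position.
; On BeginPlay it moves MainCharacterBP to the saved transform, or creates the SaveGame1 slot if none exists.
; SaveGame stores the player's transform and always writes Puntaje (score) as zero.
; LoadGame restarts the level so BeginPlay reapplies the save; BorrarInfo deletes the slot before restarting.
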(event Custom|SaveGame
  ;[1 1 1] Guardar juego
  (bind _returnvalue (SaveGame|LoadGamefromSlot (Variables|Default|GetSlotName1)))
  (bind _assave_game_1 (Utilities|Casting|CastToSaveGame1 _returnvalue))
  (Variables|/Game/Videojuegos3D/Blueprints/SaveLoadData/SaveGame1.SaveGame1_C|SetPlayerTranform _assave_game_1 (Transformation|GetActorTransform (Game|GetPlayerCharacter 0)))
  (Variables|/Game/Videojuegos3D/Blueprints/SaveLoadData/SaveGame1.SaveGame1_C|SetPuntaje _assave_game_1 0)
  (SaveGame|SaveGametoSlot _assave_game_1 (Variables|Default|GetSlotName1)))

(event Custom|LoadGame
  (Development|ExecuteConsoleCommand "RestartLevel" 0))

(event Custom|BorrarInfo
  (SaveGame|DeleteGameinSlot (Variables|Default|GetSlotName1))
  (Development|ExecuteConsoleCommand "RestartLevel" 0))

(event EventBeginPlay
  (bind _returnvalue (SaveGame|DoesSaveGameExist (Variables|Default|GetSlotName1)))
  (if _returnvalue
    ;[1 1 1] Cargar informacion inicial
    (bind _returnvalue_2 (SaveGame|LoadGamefromSlot (Variables|Default|GetSlotName1)))
    (bind _assave_game_1 (Utilities|Casting|CastToSaveGame1 _returnvalue_2))
    (bind _asmain_character_bp (Utilities|Casting|CastToMainCharacterBP (Game|GetPlayerCharacter 0)))
    (Transformation|SetWorldTransform (Variables|/Script/Engine.Actor|GetRootComponent _asmain_character_bp) (Variables|/Game/Videojuegos3D/Blueprints/SaveLoadData/SaveGame1.SaveGame1_C|GetPlayerTranform _assave_game_1) false false)
    (else
      ;[1 1 1] Se crea por primera vez el espacio de memoria SLOT1
      (bind _returnvalue_3 (SaveGame|CreateSaveGameObject "/Game/Videojuegos3D/Blueprints/SaveLoadData/SaveGame1.SaveGame1_C"))
      (SaveGame|SaveGametoSlot _returnvalue_3 (Variables|Default|GetSlotName1)))))

(event EventTick
  (params (DeltaSeconds :type Float%20%28single-precision%29)))

(fn ConstructionScript)