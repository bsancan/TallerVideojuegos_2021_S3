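; Collectible life item that adds lives to the player character when picked up.
; On RecolectarItem it increases the character's Vidas by Cantidad and pushes the new total to the HUD.
; It then calls LimpiarMensaje to clear the message and destroys itself.
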(event EventBeginPlay
  (|CallParentFunction) ; This node is disabled and will not be called.\nDrag off pins to build functionality.
)

(event EventRecolectarItem
  (bind _characterref (Variables|Default|GetCharacterRef))
  (bind _output_get (Variables|/Game/Videojuegos3D/Blueprints/MainCharacterBP.MainCharacterBP_C|SetVidas _characterref (+ (Variables|/Game/Videojuegos3D/Blueprints/MainCharacterBP.MainCharacterBP_C|GetVidas _characterref) (Variables|Default|GetCantidad))))
  (Default|SetVidas (Variables|Default|GetHUD) _output_get)
  (CallFunction|LimpiarMensaje)
  (Actor|DestroyActor))

(fn ConstructionScript
  (|CallParentFunction))