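; ItemEspada is a sword pickup that equips the character when collected.
; RecolectarItem spawns an Espada actor, snaps it to the EspadaSocket on the character's mesh, clears the message, updates the HUD item text and destroys the pickup.
; Tick resets the Cube's relative rotation to zero every frame.
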(event EventBeginPlay
  (|CallParentFunction) ; This node is disabled and will not be called.\nDrag off pins to build functionality.
)

(event EventTick
  (params (DeltaSeconds :type Float%20%28single-precision%29))
  (Transformation|SetRelativeRotation (Variables|Default|GetCube) "0, 0, 0" false false))

(event EventRecolectarItem
  (bind _characterref (Variables|Default|GetCharacterRef))
  (bind _returnvalue (Game|SpawnActorfromClass "/Game/Videojuegos3D/Blueprints/Items/Espada.Espada_C" (Math|Transform|MakeTransform "0, 0, 0") "AdjustIfPossibleButAlwaysSpawn" (Components|GetOwner _characterref) 0))
  (Transformation|AttachComponentToComponent _returnvalue (Variables|/Script/Engine.Character|GetMesh _characterref) "EspadaSocket" "SnapToTarget" "SnapToTarget" "KeepWorld" true)
  (CallFunction|LimpiarMensaje)
  (Default|SetItem (Variables|Default|GetHUD) "Tienes 1 espada")
  (Actor|DestroyActor))

(fn ConstructionScript
  (|CallParentFunction))