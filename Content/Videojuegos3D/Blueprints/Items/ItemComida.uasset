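; ItemComida is a collectible food item that adds to the player character's food count when picked up.
; Its RecolectarItem event adds Cantidad to the character's Comida and pushes the new total to the HUD.
; It then calls LimpiarMensaje and destroys the actor.
; The file has no active overlap or tick logic, so collection runs only when that event is called.
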(event EventBeginPlay
  (|CallParentFunction) ; This node is disabled and will not be called.\nDrag off pins to build functionality.
)

(event Collision|EventActorBeginOverlap
  (params (OtherActor :type Actor%20Object%20Reference)))

(event EventTick
  (params (DeltaSeconds :type Float%20%28single-precision%29)))

(event EventRecolectarItem
  (bind _characterref (Variables|Default|GetCharacterRef))
  (bind _output_get (Variables|/Game/Videojuegos3D/Blueprints/MainCharacterBP.MainCharacterBP_C|SetComida _characterref (+ (Variables|/Game/Videojuegos3D/Blueprints/MainCharacterBP.MainCharacterBP_C|GetComida _characterref) (Variables|Default|GetCantidad))))
  (Default|SetComida (Variables|Default|GetHUD) _output_get)
  (CallFunction|LimpiarMensaje)
  (Actor|DestroyActor))

(fn ConstructionScript
  (|CallParentFunction))