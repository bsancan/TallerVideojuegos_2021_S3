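; Base Blueprint for items that show a HUD prompt when the player character approaches.
; BeginPlay fetches the HUD from MainCharacterBP, retrying on a short delay until it is valid.
; Box overlap stores the character, registers the item as that character's current Item and displays MensajeInicial; leaving clears both references and the message.
; MostarDosNombres is a stub returning an empty string, and the construction script is empty.
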(event OnComponentBeginOverlap(Box)
  (params (OverlappedComponent :type Primitive%20Component%20Object%20Reference) (OtherActor :type Actor%20Object%20Reference) (OtherComp :type Primitive%20Component%20Object%20Reference) (OtherBodyIndex :type Integer) (bFromSweep :type Boolean) (SweepResult :type Hit%20Result%20Structure%20%28by%20ref%29))
  (bind _asmain_character_bp (Utilities|Casting|CastToMainCharacterBP OtherActor))
  (Variables|Default|SetCharacterRef _asmain_character_bp)
  (Variables|/Game/Videojuegos3D/Blueprints/MainCharacterBP.MainCharacterBP_C|SetItem _asmain_character_bp self)
  (CallFunction|MostrarMensaje))

(event OnComponentEndOverlap(Box)
  (params (OverlappedComponent :type Primitive%20Component%20Object%20Reference) (OtherActor :type Actor%20Object%20Reference) (OtherComp :type Primitive%20Component%20Object%20Reference) (OtherBodyIndex :type Integer))
  (bind _asmain_character_bp (Utilities|Casting|CastToMainCharacterBP OtherActor))
  (Variables|Default|SetCharacterRef 0)
  (Variables|/Game/Videojuegos3D/Blueprints/MainCharacterBP.MainCharacterBP_C|SetItem _asmain_character_bp 0)
  (CallFunction|LimpiarMensaje))

(event EventBeginPlay
  (bind _asmain_character_bp (Utilities|Casting|CastToMainCharacterBP (Game|GetPlayerCharacter 0) :!label _label))
  (Utilities|IsValid (Variables|/Game/Videojuegos3D/Blueprints/MainCharacterBP.MainCharacterBP_C|GetHUD _asmain_character_bp)
    (:Is%20Valid
      (Variables|Default|SetHUD (Variables|/Game/Videojuegos3D/Blueprints/MainCharacterBP.MainCharacterBP_C|GetHUD _asmain_character_bp)))
    (:Is%20Not%20Valid
      (Utilities|FlowControl|Delay 0.2)
      (goto _label))))

(fn ConstructionScript)

(fn MostrarMensaje
  (Default|SetMensaje (Variables|Default|GetHUD) (Utilities|Text|ToText(String) (Variables|Parametros|GetMensajeInicial))))

(fn LimpiarMensaje
  (Default|SetMensaje (Variables|Default|GetHUD)))

(fn MostarDosNombres
  (params (Nombre :type String))
  (return ""))