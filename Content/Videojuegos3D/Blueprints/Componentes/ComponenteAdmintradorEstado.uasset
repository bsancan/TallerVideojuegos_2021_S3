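; Actor component that holds its owner's current state as an enum and broadcasts OnEstadoCambiado with the previous and new values when it changes.
; SetEstado cancels any pending SetEstadoIdle timer before storing the new state, so a fresh change overrides a scheduled reset.
; ResetEstado returns to the idle state immediately or after a delay via timer, except from one protected enum state, which it leaves untouched.
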(event EventBeginPlay)

(event EventTick
  (params (DeltaSeconds :type Float%20%28single-precision%29)))

(fn SetEstado
  (params (NuevoEstado :type E_Estado%20Enum :default "NewEnumerator0"))
  (Utilities|Time|ClearTimerbyFunctionName 0 "SetEstadoIdle")
  (LocalVariables|SetL_EstadoPrevio (Variables|Default|GetEstadoActual))
  (bind _output_get (Variables|Default|SetEstadoActual NuevoEstado))
  (if (Utilities|Enum|NotEqual(Enum) _output_get (LocalVariables|GetL_EstadoPrevio))
    (Default|CallOnEstadoCambiado (LocalVariables|GetL_EstadoPrevio) (Variables|Default|GetEstadoActual))))

(fn GetEstado
  (return (Variables|Default|GetEstadoActual)))

(fn ResetEstado
  (params (Tiempo :type Float%20%28single-precision%29))
  (if (Utilities|Enum|NotEqual(Enum) (CallFunction|GetEstado) "NewEnumerator6")
    (if (<= Tiempo 0.0)
      (Privado|SetEstadoIdle)
      (else
        (Utilities|Time|SetTimerbyEvent (EventDispatchers|CreateEvent :!event SetEstadoIdle) Tiempo)))))

(fn SetEstadoIdle
  (CallFunction|SetEstado "NewEnumerator0"))