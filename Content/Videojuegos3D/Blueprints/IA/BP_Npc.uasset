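; BP_Npc is a talkable NPC that shows an interaction message and timed dialogue on the player's HUD.
; MostarMensaje displays the prompt and sets the player as the AI controller's target, while FinalizarConversacion resets conversation state and clears it.
; EmpezarConversacion steps through speaker-named lines with a delayed ForEach macro, breakable by Skip, then releases the player's conversation flag.
; Earlier dialogue-loop variants remain disconnected in the graph.
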(event EventSkip
  ;[1 1 1] Con un for each con delay
  (Utilities|ForEachLoopwithDelayandBreak (Variables|Default|GetDialogosP2N) 2.0) ; enters at Break
)

(event EventMostarMensaje
  (params (Player :type Actor%20Object%20Reference))
  (bind _aicontrollerref (Variables|Default|GetAiControllerRef))
  (bind _asmain_character_bp (Utilities|Casting|CastToMainCharacterBP Player))
  (Default|SetMensaje (Variables|/Game/Videojuegos3D/Blueprints/MainCharacterBP.MainCharacterBP_C|GetHUD _asmain_character_bp) (Utilities|Text|ToText(String) (Variables|NPC|GetMensaje)))
  (Default|SetTarget _aicontrollerref _asmain_character_bp)
  (Default|SetInteractuar _aicontrollerref true))

(event EventEmpezarConversacion
  (params (Player :type Actor%20Object%20Reference))
  (bind _asmain_character_bp (Utilities|Casting|CastToMainCharacterBP Player))
  (if (not (Variables|Default|GetEstaConversando))
    (Variables|Default|SetEstaConversando true)
    ;[1 1 1] Con un for each con delay
    (bind _array_element (Utilities|ForEachLoopwithDelayandBreak (Variables|Default|GetDialogosP2N) 2.0)
      (:Loop%20body
        (Default|SetMensaje (Variables|/Game/Videojuegos3D/Blueprints/MainCharacterBP.MainCharacterBP_C|GetHUD _asmain_character_bp) (Utilities|Text|ToText(String) (Utilities|String|Append (Utilities|String|EnumtoString (.Nombre (Utilities|Struct|BreakPlantillaDialogo _array_element))) ": " (.Dialogo (Utilities|Struct|BreakPlantillaDialogo _array_element))))))
      (:completed
        (Development|PrintString "Termino la conversacion")
        (Utilities|FlowControl|Delay 2.0)
        (Variables|/Game/Videojuegos3D/Blueprints/MainCharacterBP.MainCharacterBP_C|SetEstaConversando _asmain_character_bp false)))))

(event EventFinalizarConversacion
  (bind _aicontrollerref (Variables|Default|GetAiControllerRef))
  (Variables|Default|SetEstaConversando false)
  (Variables|Default|SetContador 0)
  (Default|SetInteractuar _aicontrollerref false)
  (Default|SetTarget _aicontrollerref))

(fn ConstructionScript
  (|CallParentFunction))