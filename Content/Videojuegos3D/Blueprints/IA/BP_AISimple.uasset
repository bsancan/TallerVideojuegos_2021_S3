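; Simple AI pawn that either patrols or chases the player, depending on its TipoDeComportamiento setting.
; Patrol mode loops AIMoveTo between its starting location and the PuntoPatrulla component's location, pausing at each end.
; Chase mode uses AIPerception to move toward a sensed MainCharacterBP.
; An unconnected perception-free chase loop remains, along with a Mover helper wrapping AIMoveTo that these graphs never call.
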(event OnTargetPerceptionUpdated(AIPerception)
  (params (Actor :type Actor%20Object%20Reference) (Stimulus :type AI%20Stimulus%20Structure))
  ;[1 1 1] Ai perception para identificar al Player
  (if (.bSuccessfullySensed (Utilities|Struct|BreakAIStimulus Stimulus))
    (bind _asmain_character_bp (Utilities|Casting|CastToMainCharacterBP Actor))
    ;[1 1 1] Persigue al player si el COmportamiento es PERSEGUIR
    (if (Utilities|Enum|Equal(Enum) (Variables|AI|GetTipoDeComportamiento) "NewEnumerator2")
      (AI|AIMoveTo self "0, 0, 0" _asmain_character_bp 5.0 false))))

(event EventBeginPlay
  ;[1 1 1] Se activa si el Comportamiento es Patrullar
  (if (Utilities|Enum|Equal(Enum) (Variables|AI|GetTipoDeComportamiento) "NewEnumerator1")
    ;[1 1 1] Se guarda la posicion inicial y final
    (Variables|Default|SetPosicionInicial (Transformation|GetActorLocation))
    (Variables|Default|SetPosicionDestino (Transformation|GetWorldLocation (Variables|Default|GetPuntoPatrulla)))
    ;[1 1 1] Patrulla entre la posicion Inicial y Final
    (AI|AIMoveTo self (Variables|Default|GetPosicionDestino) 0 5.0 false :!label _label
      (:OnSuccess
        (Utilities|FlowControl|Delay 3.0)
        (AI|AIMoveTo self (Variables|Default|GetPosicionInicial) 0 5.0 false
          (:OnSuccess
            (Utilities|FlowControl|Delay 3.0)
            (goto _label)))))))

(event Collision|EventActorBeginOverlap
  (params (OtherActor :type Actor%20Object%20Reference)))

(event EventTick
  (params (DeltaSeconds :type Float%20%28single-precision%29)))

(fn ConstructionScript)