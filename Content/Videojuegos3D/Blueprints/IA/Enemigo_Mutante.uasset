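; Mutant enemy Blueprint that damages the player on contact and plays attack animations.
; A Box collision overlap casts the other actor to MainCharacterBP and calls TomarDano with a fixed damage amount.
; The Atacar function switches on an attack type and plays the simple punch montage from the AtaquesMontages array, returning the play result.
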(event OnComponentBeginOverlap(Box)
  (params (OverlappedComponent :type Primitive%20Component%20Object%20Reference) (OtherActor :type Actor%20Object%20Reference) (OtherComp :type Primitive%20Component%20Object%20Reference) (OtherBodyIndex :type Integer) (bFromSweep :type Boolean) (SweepResult :type Hit%20Result%20Structure%20%28by%20ref%29))
  (bind _asmain_character_bp (Utilities|Casting|CastToMainCharacterBP OtherActor))
  (Default|TomarDano _asmain_character_bp 100))

(event EventBeginPlay
  (|CallParentFunction) ; This node is disabled and will not be called.\nDrag off pins to build functionality.
)

(event Collision|EventActorBeginOverlap
  (params (OtherActor :type Actor%20Object%20Reference))
  (|CallParentFunction OtherActor) ; This node is disabled and will not be called.\nDrag off pins to build functionality.
)

(event EventTick
  (params (DeltaSeconds :type Float%20%28single-precision%29))
  (|CallParentFunction DeltaSeconds) ; This node is disabled and will not be called.\nDrag off pins to build functionality.
)

(fn ConstructionScript
  (|CallParentFunction))

(fn Atacar
  (params (TipoAtaque :type E_AI_AtaqueEspecial%20Enum :default "NewEnumerator0"))
  (switch Utilities|FlowControl|Switch|SwitchonE_AI_AtaqueEspecial TipoAtaque
    (:NewEnumerator3
      (LocalVariables|SetL_Montage (Utilities|Array|Get(acopy) (Variables|Ataques|GetAtaquesMontages)))
      (bind _returnvalue (Animation|PlayAnimMontage (LocalVariables|GetL_Montage) 1.0 "None"))
      (return _returnvalue))))