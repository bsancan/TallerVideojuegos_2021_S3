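; Input buffer component that holds one key while the buffer is open and releases it when the buffer closes.
; A new key replaces the stored one and is consumed immediately if the buffer is closed.
; Consuming broadcasts the stored key through an event dispatcher, then resets it to the first enum value.
; Opening and closing fire their own dispatchers, and closing also triggers consumption.
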(fn ActualizarKey
  (params (NuevoKey :type E_BuferEntrada%20Enum :default "NewEnumerator0"))
  (Variables|Default|SetKeyAlmacenado NuevoKey)
  (if (not (Variables|Default|GetEstaAbierto))
    (CallFunction|ConsumirBuferEntrada)))

(fn ConsumirBuferEntrada
  (Default|CallOnBuferEntradaConsumido (Variables|Default|GetKeyAlmacenado))
  (Variables|Default|SetKeyAlmacenado "NewEnumerator0"))

(fn CerrarBuferEntrada
  (Variables|Default|SetEstaAbierto false)
  (Default|CallOnBuferEntradaCerrado)
  (CallFunction|ConsumirBuferEntrada))

(fn AbrirBuferEntrada
  (Variables|Default|SetEstaAbierto true)
  (Default|CallOnBuferEntradaAbierto))

(fn GetKeyAlmacenado
  (return (Variables|Default|GetKeyAlmacenado)))