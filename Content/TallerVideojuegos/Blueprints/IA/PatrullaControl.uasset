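; PatrullaControl is an AI patrol helper actor that holds a list of patrol points in PuntosPatrulla.
; GetPuntoPatrulla returns the point at a given index after checking that the array is not empty and the index does not exceed the last element.
; The event graph and construction script are empty, so it acts only as a data holder with that lookup.
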(event EventBeginPlay)

(event Collision|EventActorBeginOverlap
  (params (OtherActor :type Actor%20Object%20Reference)))

(event EventTick
  (params (DeltaSeconds :type Float%20%28single-precision%29)))

(fn ConstructionScript)

(fn GetPuntoPatrulla
  (params (Index :type Integer))
  (if (> (Utilities|Array|Length (Variables|Patrulla|GetPuntosPatrulla)) 0)
    (if (<= Index (- (Utilities|Array|Length (Variables|Patrulla|GetPuntosPatrulla)) 1))
      (return (Utilities|Array|Get(acopy) (Variables|Patrulla|GetPuntosPatrulla) Index)))))