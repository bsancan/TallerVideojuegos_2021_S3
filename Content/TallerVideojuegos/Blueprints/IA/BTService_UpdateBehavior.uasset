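; BTService_UpdateBehavior is a Behavior Tree service that selects the current behavior state for an AI pawn derived from BP_AIBase.
; It caches the controlled pawn on search start, then on each tick writes one of three enum states to the behavior Blackboard key.
; A valid target actor takes priority; otherwise the state depends on whether the pawn has a valid PatrullaControl (patrol control) reference.
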(event EventReceiveSearchStartAI
  (params (OwnerController :type AI%20Controller%20Object%20Reference) (ControlledPawn :type Pawn%20Object%20Reference))
  (bind _asbp_aibase (Utilities|Casting|CastToBP_AIBase ControlledPawn))
  (Variables|Default|SetBP_AIBase _asbp_aibase))

(event EventReceiveTickAI
  (params (OwnerController :type AI%20Controller%20Object%20Reference) (ControlledPawn :type Pawn%20Object%20Reference) (DeltaSeconds :type Float%20%28single-precision%29))
  (Variables|Default|GetBP_AIBase
    (:then
      (bind _output_get (Variables|Default|SetTargetActor (AI|BehaviorTree|GetBlackboardValueasActor (Variables|Default|GetTargetKey))))
      (Utilities|IsValid _output_get
        (:Is%20Valid
          (Utilities|SetBehavior "NewEnumerator2"))
        (:Is%20Not%20Valid
          (Variables|/Game/TallerVideojuegos/Blueprints/IA/BP_AIBase.BP_AIBase_C|GetPatrullaControl (Variables|Default|GetBP_AIBase)
            (:then
              (Utilities|SetBehavior "NewEnumerator1"))
            (:else
              (Utilities|SetBehavior "NewEnumerator0"))))))
    (:else)))