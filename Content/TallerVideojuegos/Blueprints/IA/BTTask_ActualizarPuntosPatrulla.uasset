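; Behavior Tree task that advances an AI character's patrol point index in the Blackboard.
; It casts the controlled pawn to BP_AIBase and reads the patrol point array from its PatrullaControl reference.
; The PatrullaIndex key increments until the last point, then wraps to zero, and the task finishes successfully.
; If the cast fails or PatrullaControl is invalid, the task never calls FinishExecute.
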(event EventReceiveExecuteAI
  (params (OwnerController :type AI%20Controller%20Object%20Reference) (ControlledPawn :type Pawn%20Object%20Reference))
  (bind _asbp_aibase (Utilities|Casting|CastToBP_AIBase ControlledPawn))
  (bind _patrullacontrol (Variables|/Game/TallerVideojuegos/Blueprints/IA/BP_AIBase.BP_AIBase_C|GetPatrullaControl _asbp_aibase)
    (:then
      (if (> (Utilities|Array|Length (Variables|/Game/TallerVideojuegos/Blueprints/IA/PatrullaControl.PatrullaControl_C|GetPuntosPatrulla _patrullacontrol)) (+ (Class|BTFunctionLibrary|GetBlackboardValueasInt (Variables|Default|GetPatrullaIndex)) 1))
        (Class|BTFunctionLibrary|SetBlackboardValueasInt (Variables|Default|GetPatrullaIndex) (+ (Class|BTFunctionLibrary|GetBlackboardValueasInt (Variables|Default|GetPatrullaIndex)) 1))
        (AI|BehaviorTree|FinishExecute true)
        (else
          (Class|BTFunctionLibrary|SetBlackboardValueasInt (Variables|Default|GetPatrullaIndex))
          (AI|BehaviorTree|FinishExecute true))))
    (:else)))