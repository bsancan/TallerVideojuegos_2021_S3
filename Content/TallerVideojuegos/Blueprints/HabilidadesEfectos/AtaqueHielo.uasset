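; AtaqueHielo is an ice attack effect actor with a timed hit area.
; On BeginPlay it turns its Sphere collision off, enables it as query-only after a short delay, then disables it again before destroying itself.
; The sequence runs on chained Delays through two custom events that toggle collision.
; The graph contains no overlap, damage or movement logic.
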(event Custom|DesactivarCollision
  (Collision|SetCollisionEnabled (Variables|Default|GetSphere) "NoCollision"))

(event Custom|ActivarCollision
  (Collision|SetCollisionEnabled (Variables|Default|GetSphere) "QueryOnly"))

(event EventBeginPlay
  (CallFunction|DesactivarCollision)
  (Utilities|FlowControl|Delay 0.5)
  (CallFunction|ActivarCollision)
  (Utilities|FlowControl|Delay 3.0)
  (CallFunction|DesactivarCollision)
  (Utilities|FlowControl|Delay 1.0)
  (Actor|DestroyActor))

(event Collision|EventActorBeginOverlap
  (params (OtherActor :type Actor%20Object%20Reference)))

(event EventTick
  (params (DeltaSeconds :type Float%20%28single-precision%29)))

(fn ConstructionScript)